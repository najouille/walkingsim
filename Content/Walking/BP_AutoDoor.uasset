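; BP_AutoDoor is a sliding double door that opens and closes automatically in the walking part of the game.
; Overlapping the DetectionZone plays a 2D sound and slides DoorL and DoorR apart with eased MoveComponentTo calls.
; Ending the overlap plays a closing sound and slides both panels back together.
; The overlap events do not filter actors or count occupants, so any exit triggers closing.
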(event `self.ReceiveBeginPlay`)

(event `self.DetectionZone.OnComponentBeginOverlap`
  (params (OverlappedComponent :type "PrimitiveComponent Object Reference") (OtherActor :type "Actor Object Reference") (OtherComp :type "PrimitiveComponent Object Reference") (OtherBodyIndex :type Integer) (bFromSweep :type Boolean) (SweepResult :type "HitResult Structure (by ref)"))
  (`GameplayStatics.PlaySound2D` null 1.0 1.0 0.0 null null)
  (`|ExecutionSequence`
    (:`then_0`
      (`KismetSystemLibrary.MoveComponentTo` (`self.Door_L`) (-146.0 0.0 100.0) (struct) true false 0.4))
    (:`then_1`
      (`KismetSystemLibrary.MoveComponentTo` (`self.Door_R`) (146.0 0.0 100.0) (struct) true false 0.4))))

(event `self.DetectionZone.OnComponentEndOverlap`
  (params (OverlappedComponent :type "PrimitiveComponent Object Reference") (OtherActor :type "Actor Object Reference") (OtherComp :type "PrimitiveComponent Object Reference") (OtherBodyIndex :type Integer))
  (`GameplayStatics.PlaySound2D` "/Engine/VREditor/Sounds/UI/Dockable_Window_Close.Dockable_Window_Close" 1.0 1.0 0.0 null null)
  (`|ExecutionSequence`
    (:`then_0`
      (`KismetSystemLibrary.MoveComponentTo` (`self.Door_L`) (-50.0 0.0 100.0) (struct) true false 0.4))
    (:`then_1`
      (`KismetSystemLibrary.MoveComponentTo` (`self.Door_R`) (50.0 0.0 100.0) (struct) true false 0.4))))

(fn `UserConstructionScript`)