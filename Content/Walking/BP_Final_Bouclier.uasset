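; BP_Final_Bouclier is a card-gated terminal that acts as an apparent placeholder for the "Fin Famille" ending.
; On player overlap it shows an interact widget if the game controller's CarteBleuh is set, and a CardNeeded widget if the character's Cartes lack ValCarte.
; End overlap removes one widget according to CarteBleuh.
; The Elevator input only prints "Fin Famille" while InBox is set, which overlap does regardless of card ownership.
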(event `InputAction|Elevator`
  (params (Key :type "Key Structure"))
  (:`Pressed`
    (if true
      (bind _output_get (set `self.Epressed` true))
      (if (and _output_get (stale `self.Terminal.OnComponentBeginOverlap` _output_get))
        (`KismetSystemLibrary.PrintString` "Fin Famille")))))

(event `self.Terminal.OnComponentBeginOverlap`
  (params (OverlappedComponent :type "PrimitiveComponent Object Reference") (OtherActor :type "Actor Object Reference") (OtherComp :type "PrimitiveComponent Object Reference") (OtherBodyIndex :type Integer) (bFromSweep :type Boolean) (SweepResult :type "HitResult Structure (by ref)"))
  (bind _asbp_story_adv_character (cast `/Game/TPSAT/Blueprints/Character/BP_StoryAdv_Character` OtherActor))
  (`|ExecutionSequence`
    (:`then_0`
      (`self.InteractUI`)
      (bind _output_get (set `self.InBox` true)))
    (:`then_1`
      (`/Engine/EditorBlueprintResources/StandardMacros.DoOnce` false :!label _label
        (:`Completed`
          (for (_array_element _array_index) (`/Game/TPSAT/Blueprints/Character/BP_StoryAdv_Character.Cartes` _asbp_story_adv_character)
            (bind _returnvalue (and _array_element (== _array_index (`self.ValCarte`))))
            (if _returnvalue
              (`self.InteractUI`)
              (break)))
          (if (not _returnvalue)
            (`|ExecutionSequence`
              (:`then_0`
                (`/Engine/EditorBlueprintResources/StandardMacros.DoOnce` false :!label _label_2
                  (:`Completed`
                    (bind _returnvalue_2 (`|CreateWidget` "/Game/Walking/Blueprints/CardNeeded.CardNeeded_C"))
                    (`UserWidget.AddToViewport` _returnvalue_2 0)
                    (goto _label_2 :!via `Reset`))))
              (:`then_1`
                (goto _label :!via `Reset`)))))))))

(event `self.Terminal.OnComponentEndOverlap`
  (params (OverlappedComponent :type "PrimitiveComponent Object Reference") (OtherActor :type "Actor Object Reference") (OtherComp :type "PrimitiveComponent Object Reference") (OtherBodyIndex :type Integer))
  (cast `/Game/TPSAT/Blueprints/Character/BP_StoryAdv_Character` OtherActor)
  (if (`/Game/TPSAT/Blueprints/Core/BP_StoryAdv_GameController.carteBleuh` (`/Game/TPSAT/Blueprints/Core/BP_StoryAdv_FunctionLibrary.GetGameController`))
    (`Widget.RemoveFromParent` (stale `InteractUI` _returnvalue))
    (set `self.InBox` false)
    (else
      (`Widget.RemoveFromParent` (stale `self.Terminal.OnComponentBeginOverlap` _returnvalue_2)))))

(event `InteractUI`
  (if (`/Game/TPSAT/Blueprints/Core/BP_StoryAdv_GameController.carteBleuh` (`/Game/TPSAT/Blueprints/Core/BP_StoryAdv_FunctionLibrary.GetGameController`))
    (`/Engine/EditorBlueprintResources/StandardMacros.DoOnce` false :!label _label_3
      (:`Completed`
        (`self.EnableInput` (`GameplayStatics.GetPlayerController` 0))
        (bind _returnvalue (`|CreateWidget` "/Game/Walking/InteractUI.InteractUI_C"))
        (`UserWidget.AddToViewport` _returnvalue 0)
        (goto _label_3 :!via `Reset`)))))

(fn `UserConstructionScript`)