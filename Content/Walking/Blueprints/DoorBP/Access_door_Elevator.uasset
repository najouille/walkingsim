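; Card-locked elevator access door whose two sliding panels open on the Elevator input once the player holds the required card.
; Overlapping the terminal checks the character's Cartes array at ValCarte, then either sets PossCard and enables input or warns that a card is needed.
; The detection zone prompts for a card on entry, and on exit disables input and slides the panels back.
; DoOnce gates throttle the timed UI widgets.
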(event `self.DetectionZone.OnComponentEndOverlap`
  (params (OverlappedComponent :type "PrimitiveComponent Object Reference") (OtherActor :type "Actor Object Reference") (OtherComp :type "PrimitiveComponent Object Reference") (OtherBodyIndex :type Integer))
  (`self.DisableInput` (`GameplayStatics.GetPlayerController` 0))
  (`GameplayStatics.PlaySound2D` "/Game/Walking/Blueprints/DoorBP/DoorOpening.DoorOpening" 1.0 1.0 0.0 null null)
  (`|ExecutionSequence`
    (:`then_0`
      (`KismetSystemLibrary.MoveComponentTo` (`self.Door_L`) (-50.0 0.0 100.0) (struct) true false 1.0))
    (:`then_1`
      (`KismetSystemLibrary.MoveComponentTo` (`self.Door_R`) (50.0 0.0 100.0) (struct) true false 1.0))))

(event `InputAction|Elevator`
  (params (Key :type "Key Structure"))
  (:`Pressed`
    (`GameplayStatics.PlaySound2D` "/Game/Walking/Blueprints/DoorOpening.DoorOpening" 1.0 1.0 0.0 null null)
    (`|ExecutionSequence`
      (:`then_0`
        (`KismetSystemLibrary.MoveComponentTo` (`self.Door_L`) (-146.0 0.0 100.0) (struct) true false 3.0))
      (:`then_1`
        (`KismetSystemLibrary.MoveComponentTo` (`self.Door_R`) (146.0 0.0 100.0) (struct) true false 3.0)))))

(event `self.Terminal.OnComponentBeginOverlap`
  (params (OverlappedComponent :type "PrimitiveComponent Object Reference") (OtherActor :type "Actor Object Reference") (OtherComp :type "PrimitiveComponent Object Reference") (OtherBodyIndex :type Integer) (bFromSweep :type Boolean) (SweepResult :type "HitResult Structure (by ref)"))
  (bind _asbp_story_adv_character (cast `/Game/TPSAT/Blueprints/Character/BP_StoryAdv_Character` OtherActor))
  (`|ExecutionSequence`
    (:`then_0`
      (`self.InteractUI`))
    (:`then_1`
      (`/Engine/EditorBlueprintResources/StandardMacros.DoOnce` false :!label _label
        (:`Completed`
          (for (_array_element _array_index) (`/Game/TPSAT/Blueprints/Character/BP_StoryAdv_Character.Cartes` _asbp_story_adv_character)
            (bind _returnvalue (and _array_element (== _array_index (`self.ValCarte`))))
            (if _returnvalue
              (set `self.PossCard` true)
              (`self.InteractUI`)
              (break)))
          (if (not _returnvalue)
            (`|ExecutionSequence`
              (:`then_0`
                (`/Engine/EditorBlueprintResources/StandardMacros.DoOnce` false :!label _label_2
                  (:`Completed`
                    (bind _returnvalue_2 (`|CreateWidget` "/Game/Walking/Blueprints/CardNeeded.CardNeeded_C"))
                    (`UserWidget.AddToViewport` _returnvalue_2 0)
                    (`KismetSystemLibrary.Delay` 4.0)
                    (`Widget.RemoveFromParent` _returnvalue_2)
                    (goto _label_2 :!via `Reset`))))
              (:`then_1`
                (goto _label :!via `Reset`)))))))))

(event `self.DetectionZone.OnComponentBeginOverlap`
  (params (OverlappedComponent :type "PrimitiveComponent Object Reference") (OtherActor :type "Actor Object Reference") (OtherComp :type "PrimitiveComponent Object Reference") (OtherBodyIndex :type Integer) (bFromSweep :type Boolean) (SweepResult :type "HitResult Structure (by ref)"))
  (cast `/Game/TPSAT/Blueprints/Character/BP_StoryAdv_Character` OtherActor)
  (if (not (`self.PossCard`))
    (`/Engine/EditorBlueprintResources/StandardMacros.DoOnce` false :!label _label_3
      (:`Completed`
        (bind _returnvalue (`|CreateWidget` "/Game/Walking/Blueprints/Inserer_carte.Inserer_carte_C"))
        (`UserWidget.AddToViewport` _returnvalue 0)
        (`KismetSystemLibrary.Delay` 2.0)
        (`Widget.RemoveFromParent` _returnvalue)
        (goto _label_3 :!via `Reset`)))))

(event `InteractUI`
  (if (`self.PossCard`)
    (`/Engine/EditorBlueprintResources/StandardMacros.DoOnce` false :!label _label_4
      (:`Completed`
        (`self.EnableInput` (`GameplayStatics.GetPlayerController` 0))
        (bind _returnvalue (`|CreateWidget` "/Game/Walking/InteractUI.InteractUI_C"))
        (`UserWidget.AddToViewport` _returnvalue 0)
        (`KismetSystemLibrary.Delay` 4.0)
        (`Widget.RemoveFromParent` _returnvalue)
        (goto _label_4 :!via `Reset`)))))

(fn `UserConstructionScript`)