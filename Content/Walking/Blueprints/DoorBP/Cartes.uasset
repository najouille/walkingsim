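; Keycard pickup actor that records a found card on the adventure character when the player walks into its trigger box.
; On overlap it inserts a true entry into the character's Cartes array at the card's ValCarte index and removes its box and CarteB component.
; A CarteTrouvee widget shows for two seconds, then the actor destroys itself.
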(event `self.Box.OnComponentBeginOverlap`
  (params (OverlappedComponent :type "PrimitiveComponent Object Reference") (OtherActor :type "Actor Object Reference") (OtherComp :type "PrimitiveComponent Object Reference") (OtherBodyIndex :type Integer) (bFromSweep :type Boolean) (SweepResult :type "HitResult Structure (by ref)"))
  (bind _asbp_story_adv_character (cast `/Game/TPSAT/Blueprints/Character/BP_StoryAdv_Character` OtherActor))
  (`KismetArrayLibrary.Array_Insert` (`/Game/TPSAT/Blueprints/Character/BP_StoryAdv_Character.Cartes` _asbp_story_adv_character) true (`self.ValCarte`))
  (bind _returnvalue (`|CreateWidget` "/Game/Walking/Blueprints/CarteTrouvee.CarteTrouvee_C"))
  (`UserWidget.AddToViewport` _returnvalue 0)
  (`ActorComponent.K2_DestroyComponent` (`self.Box`))
  (`ActorComponent.K2_DestroyComponent` (`self.CarteB`))
  (`KismetSystemLibrary.Delay` 2.0)
  (`Widget.RemoveFromParent` _returnvalue)
  (`self.K2_DestroyActor`))

(fn `UserConstructionScript`)