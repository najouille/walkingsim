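; Test Blueprint for a double sliding door that opens when something enters its Detection volume and closes when it leaves.
; Both overlap events slide DoorL and DoorR to fixed relative positions with eased MoveComponentTo calls, alongside 2D sound calls.
; A timeline-driven OpenDoor event with positional sound is called only from disconnected keycard logic, which checks the character's Cartes and otherwise briefly shows a CardNeeded widget.
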(event `self.Detection.OnComponentEndOverlap`
  (params (OverlappedComponent :type "PrimitiveComponent Object Reference") (OtherActor :type "Actor Object Reference") (OtherComp :type "PrimitiveComponent Object Reference") (OtherBodyIndex :type Integer))
  (`GameplayStatics.PlaySound2D` "/Engine/VREditor/Sounds/UI/Dockable_Window_Close.Dockable_Window_Close" 1.0 1.0 0.0 null null)
  (`|ExecutionSequence`
    (:`then_0`
      (`KismetSystemLibrary.MoveComponentTo` (`self.DoorL`) (-50.0 0.0 100.0) (struct) true false 0.4))
    (:`then_1`
      (`KismetSystemLibrary.MoveComponentTo` (`self.DoorR`) (50.0 0.0 100.0) (struct) true false 0.4))))

(event `OpenDoor`
  (`GameplayStatics.PlaySoundAtLocation` "/Game/Walking/Blueprints/DoorBP/DoorOpening.DoorOpening" (`self.K2_GetActorLocation`) (struct) 1.0 1.0 0.8 null null null null)
  (bind (_direction _opendoorr _opendoorl) (`Timeline|doorOpen` :!via `PlayFromStart`)
    (:`Update`
      (`|ExecutionSequence`
        (:`then_0`
          (`SceneComponent.K2_SetRelativeLocation` (`self.DoorL`) (`KismetMathLibrary.VLerp` (`self.ClosedL`) (`self.OpenL`) _opendoorl) false false))
        (:`then_1`
          (`SceneComponent.K2_SetRelativeLocation` (`self.DoorR`) (`KismetMathLibrary.VLerp` (`self.ClosedR`) (`self.OpenR`) _opendoorr) false false))))))

(event `self.Detection.OnComponentBeginOverlap`
  (params (OverlappedComponent :type "PrimitiveComponent Object Reference") (OtherActor :type "Actor Object Reference") (OtherComp :type "PrimitiveComponent Object Reference") (OtherBodyIndex :type Integer) (bFromSweep :type Boolean) (SweepResult :type "HitResult Structure (by ref)"))
  (`GameplayStatics.PlaySound2D` null 1.0 1.0 0.0 null null)
  (`|ExecutionSequence`
    (:`then_0`
      (`KismetSystemLibrary.MoveComponentTo` (`self.DoorL`) (-146.0 0.0 100.0) (struct) true false 0.4))
    (:`then_1`
      (`KismetSystemLibrary.MoveComponentTo` (`self.DoorR`) (146.0 0.0 100.0) (struct) true false 0.4))))

(fn `UserConstructionScript`)