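; BP_Reference scatters a grid of instanced reference dummy meshes over whatever surfaces lie beneath it.
; RefreshGrid clears the instances, sets the mesh, then steps across GridSize at Gap spacing, centered on the world origin rather than the actor.
; Each point fires a debug-drawn vertical Visibility trace and adds a world-space instance at any hit location.
; ClearGrid removes all instances, and the construction script is empty.
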(event `ClearGrid`
  (`InstancedStaticMeshComponent.ClearInstances` (`self.DummyMesh`)))

(event `RefreshGrid`
  (bind (_gridsize_x _gridsize_y) (`KismetMathLibrary.BreakVector2D` (`self.GridSize`)))
  (bind _gap (`self.Gap`))
  (bind _gap_2 (`self.Gap`))
  (bind _traceheight (`self.TraceHeight`))
  (bind _dummymesh (`self.DummyMesh`))
  (bind _returnvalue (/ _gridsize_x 2.0 _gap))
  (bind _returnvalue_2 (/ _gridsize_y 2.0 _gap))
  (`InstancedStaticMeshComponent.ClearInstances` _dummymesh)
  (`StaticMeshComponent.SetStaticMesh` _dummymesh (`self.SM_RefDummyMesh`))
  (for _index (range (`KismetMathLibrary.FTrunc` (* _returnvalue -1.0)) (+ (`KismetMathLibrary.FTrunc` _returnvalue) 1))
    (for _index_2 (range (`KismetMathLibrary.FTrunc` (* _returnvalue_2 -1.0)) (+ (`KismetMathLibrary.FTrunc` _returnvalue_2) 1))
      (bind _returnvalue_3 (* _index _gap_2))
      (bind _returnvalue_4 (* _index_2 _gap_2))
      (bind (_outhit _returnvalue_5) (`KismetSystemLibrary.LineTraceSingle` :`Start` (`KismetMathLibrary.MakeVector` _returnvalue_3 _returnvalue_4 _traceheight) :`End` (`KismetMathLibrary.MakeVector` _returnvalue_3 _returnvalue_4 (* _traceheight -1.0)) :`TraceChannel` "TraceTypeQuery1" :`DrawDebugType` "ForDuration"))
      (if _returnvalue_5
        (`InstancedStaticMeshComponent.AddInstance` (`self.DummyMesh`) (`KismetMathLibrary.Conv_VectorToTransform` (`.Location` (`GameplayStatics.BreakHitResult` _outhit))) true)))))

(fn `UserConstructionScript`)